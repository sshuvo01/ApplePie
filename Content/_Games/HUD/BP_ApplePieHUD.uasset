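; HUD Blueprint that draws a dynamic four-piece crosshair for the player's BP_ApplePieCharacter.
; BeginPlay caches the player pawn as that character, printing an error if the cast fails.
; Each DrawHUD offsets the screen center, reads the character's crosshair spread, and pushes the top, bottom, left and right textures outward in proportion to it.
; An invalid character prints a message instead of drawing.
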(event EventBeginPlay
  (bind _asbp_apple_pie_character (Utilities|Casting|CastToBP_ApplePieCharacter (Game|Player|GetPlayerPawn 0))
    (:then
      (Variables|Bork|SetCharacter _asbp_apple_pie_character))
    (:CastFailed
      (Development|PrintString "Cast failed"))))

(event Collision|EventActorBeginOverlap
  (params (OtherActor :type Actor%20Object%20Reference)))

(event EventTick
  (params (DeltaSeconds :type Float%20%28single-precision%29)))

(event EventDrawHUD
  (params (SizeX :type Integer) (SizeY :type Integer))
  ;[1 1 1] Calculating screen center
  (Variables|Bork|SetScreenCenter (Math|Vector2D|MakeVector2D (/ (Math|Conversions|ToFloat(Integer) SizeX) 2.0) (/ (Math|Conversions|ToFloat(Integer) SizeY) 2.0)))
  ;[1 1 1] Calculating crosshair location
  (Variables|Bork|SetCrosshairLocation (Math|Vector2D|MakeVector2D (+ (.x (Variables|Bork|GetScreenCenter)) (Variables|Bork|GetCrosshairOffxetX)) (+ (.y (Variables|Bork|GetScreenCenter)) (Variables|Bork|GetCrosshairOffxetY))))
  ;[1 1 1] Getting crosshair spread
  (Utilities|IsValid (Variables|Bork|GetCharacter)
    (:Is%20Valid
      (Variables|Bork|SetCrosshairSpreadMultiplier (Class|ApplePieCharacter|GetCrosshairSpread (Variables|Bork|GetCharacter)))
      ;[1 1 1] Crosshair draw location
      (Variables|Bork|SetCrosshairDrawLocation (Math|Vector2D|MakeVector2D (- (.x (Variables|Bork|GetCrosshairLocation)) (Variables|Bork|GetCrosshairHalfW)) (- (.y (Variables|Bork|GetCrosshairLocation)) (Variables|Bork|GetCrosshairHalfH))))
      ;[1 1 1] Bottom
      (Canvas|DrawTexture "/Game/_Games/Assets/Textures/Crosshairs/Crosshair_Quad_9_Bottom.Crosshair_Quad_9_Bottom" (.x (+ (Variables|Bork|GetCrosshairDrawLocation) (Math|Vector2D|MakeVector2D 0.0 (* (Variables|Bork|GetCrosshairSpreadMultiplier) (Variables|Bork|GetCrosshairDislocationMultiplier))))) (.y (+ (Variables|Bork|GetCrosshairDrawLocation) (Math|Vector2D|MakeVector2D 0.0 (* (Variables|Bork|GetCrosshairSpreadMultiplier) (Variables|Bork|GetCrosshairDislocationMultiplier))))) 64.0 64.0 0.0 0.0 1.0 1.0 "(R=1.000000,G=1.000000,B=1.000000,A=1.000000)")
      ;[1 1 1] Top
      (Canvas|DrawTexture "/Game/_Games/Assets/Textures/Crosshairs/Crosshair_Quad_9_Top.Crosshair_Quad_9_Top" (.x (+ (Variables|Bork|GetCrosshairDrawLocation) (Math|Vector2D|MakeVector2D 0.0 (* (Variables|Bork|GetCrosshairSpreadMultiplier) (Variables|Bork|GetCrosshairDislocationMultiplier) -1.0)))) (.y (+ (Variables|Bork|GetCrosshairDrawLocation) (Math|Vector2D|MakeVector2D 0.0 (* (Variables|Bork|GetCrosshairSpreadMultiplier) (Variables|Bork|GetCrosshairDislocationMultiplier) -1.0)))) 64.0 64.0 0.0 0.0 1.0 1.0 "(R=1.000000,G=1.000000,B=1.000000,A=1.000000)")
      ;[1 1 1] Left
      (Canvas|DrawTexture "/Game/_Games/Assets/Textures/Crosshairs/Crosshair_Quad_9_Left.Crosshair_Quad_9_Left" (.x (+ (Variables|Bork|GetCrosshairDrawLocation) (Math|Vector2D|MakeVector2D (* (Variables|Bork|GetCrosshairSpreadMultiplier) (Variables|Bork|GetCrosshairDislocationMultiplier) -1.0) 0.0))) (.y (+ (Variables|Bork|GetCrosshairDrawLocation) (Math|Vector2D|MakeVector2D (* (Variables|Bork|GetCrosshairSpreadMultiplier) (Variables|Bork|GetCrosshairDislocationMultiplier) -1.0) 0.0))) 64.0 64.0 0.0 0.0 1.0 1.0 "(R=1.000000,G=1.000000,B=1.000000,A=1.000000)")
      ;[1 1 1] Right
      (Canvas|DrawTexture "/Game/_Games/Assets/Textures/Crosshairs/Crosshair_Quad_9_Right.Crosshair_Quad_9_Right" (.x (+ (Variables|Bork|GetCrosshairDrawLocation) (Math|Vector2D|MakeVector2D (* (Variables|Bork|GetCrosshairSpreadMultiplier) (Variables|Bork|GetCrosshairDislocationMultiplier) 1.0) 0.0))) (.y (+ (Variables|Bork|GetCrosshairDrawLocation) (Math|Vector2D|MakeVector2D (* (Variables|Bork|GetCrosshairSpreadMultiplier) (Variables|Bork|GetCrosshairDislocationMultiplier) 1.0) 0.0))) 64.0 64.0 0.0 0.0 1.0 1.0 "(R=1.000000,G=1.000000,B=1.000000,A=1.000000)"))
    (:Is%20Not%20Valid
      (Development|PrintString "character invalid"))))

(fn ConstructionScript)